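; A clickable 2D sprite button that tells a Lair to make a tortoise when pressed.
; BeginPlay enables click events on the first player controller, hides the mouse cursor and sets the idle sprite.
; Clicking the PaperSprite swaps to the pressed sprite and calls MakeTortoise on the Lair reference, and releasing it returns to idle through the Idle event.
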(event OnReleased(PaperSprite)
  (params (TouchedComponent :type Primitive%20Component%20Object%20Reference) (ButtonReleased :type Key%20Structure :default "None"))
  (CallFunction|EventIdle))

(event OnClicked(PaperSprite)
  (params (TouchedComponent :type Primitive%20Component%20Object%20Reference) (ButtonPressed :type Key%20Structure :default "None"))
  (Rendering|Components|Sprite|SetSprite (Variables|Default|GetPaperSprite) (Variables|Sprites|GetPressed%20On%20Sprite))
  (Default|MakeTortoise (Variables|Default|GetLair)))

(event Custom|Event%20Idle
  (Rendering|Components|Sprite|SetSprite (Variables|Default|GetPaperSprite) (Variables|Sprites|GetIdle%20Sprite)))

(event EventBeginPlay
  (bind _returnvalue (Game|GetPlayerController 0))
  (Variables|/Script/Engine.PlayerController|SetbEnableClickEvents _returnvalue true)
  (Variables|/Script/Engine.PlayerController|SetbShowMouseCursor _returnvalue false)
  (CallFunction|EventIdle))

(fn ConstructionScript)