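; Short-lived flipbook effect actor that shows an enter, exit or cherry particle animation, then destroys itself.
; Init stores a Type, which Tick switches on to call the matching event, with exit as the default.
; Each event sets the Paper flipbook and actor scale, and a per-type Delay on Tick times the actor's destruction.
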(event Custom|Event%20CherryParticle
  (Sprite|SetFlipbook (Variables|Default|GetPaperFlipbook) "/Game/SunnyLandAssets/sprites/cherry/cherry.cherry")
  (Transformation|SetActorScale3D "0.400000,1.000000,0.400000"))

(event Custom|Event%20EnterParticle
  (Sprite|SetFlipbook (Variables|Default|GetPaperFlipbook) "/Game/SunnyLandAssets/sprites/enemy-death/start.start")
  (Transformation|SetActorScale3D "1.000000,1.000000,1.000000"))

(event Custom|Event%20ExitParticle
  (Sprite|SetFlipbook (Variables|Default|GetPaperFlipbook) "/Game/SunnyLandAssets/sprites/item-feedback/finish.finish")
  (Transformation|SetActorScale3D "1.000000,1.000000,1.000000"))

(event EventTick
  (params (DeltaSeconds :type Float%20%28single-precision%29))
  (switch int (Variables|Default|GetType)
    (:Default
      (CallFunction|EventExitParticle)
      (Utilities|FlowControl|Delay 1.5))
    (:1
      (CallFunction|EventEnterParticle)
      (Utilities|FlowControl|Delay 1.5))
    (:2
      (CallFunction|EventCherryParticle)
      (Utilities|FlowControl|Delay 1.0)))
  (Actor|DestroyActor))

(fn ConstructionScript)

(fn Init
  (params (Type :type Integer))
  (Variables|Default|SetType Type))