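; Tortoise actor with a flipbook sprite that moves along X toward an EndGoal actor, then plays an end sound and despawns.
; A Tick countdown toggles State, which with Type sets speed and sprite: type 1 runs steadily, type 2 pauses periodically, type 3 periodically reverses.
; While moving, a second timer plays footstep cues, with a faster dungeon sound for type 3.
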(event Custom|Event%20Despawn
  (Audio|PlaySoundatLocation "/Game/Sounds/end.end" (Transformation|GetActorLocation) "0, 0, 0" 1.0 1.0 0.0 0 0 0 0)
  (Actor|DestroyActor))

(event EventBeginPlay
  (Audio|PlaySoundatLocation "/Game/Sounds/spawn.spawn" (Transformation|GetActorLocation) "0, 0, 0" 1.0 1.0 0.0 0 0 0 0)
  (Transformation|SetRelativeRotation (Variables|Default|GetSprite) "0.000000,180.000000,0.000000" false false))

(event EventTick
  (params (DeltaSeconds :type Float%20%28single-precision%29))
  (bind _output_get (Variables|Default|SetTime (- (Variables|Default|GetTime) DeltaSeconds)))
  (bind _speed (CallFunction|GetNewSpeed))
  (Transformation|AddRelativeLocation (Variables|Collision|GetCapsuleComponent) (* _speed DeltaSeconds (Math|Vector|MakeVector 1.0 0.0 0.0)) false false)
  (if (== _speed 0.0)
    _
    (else
      (CallFunction|UpdateSoundTime DeltaSeconds)))
  (if (< _output_get 0.0)
    (CallFunction|UpdateState)
    (CallFunction|UpdateSprite)
    (CallFunction|ResetTime))
  (bind _distanceleft (CallFunction|GetDistanceLeft))
  (if (< _distanceleft 1.0)
    (CallFunction|EventDespawn)))

(fn ConstructionScript)

(fn Init
  (params (Type :type Integer) (EndGoal :type Lair%20Object%20Reference))
  (Variables|Default|SetType Type)
  (Variables|Default|SetEndGoal EndGoal)
  (Variables|Default|SetState false)
  (Variables|Default|SetSoundTime 0.5)
  (Variables|Default|SetBaseSpeed 6e+01)
  (Variables|Default|SetTime 1.0))

(fn UpdateSprite
  (bind _sprite (Variables|Default|GetSprite))
  (bind _type (Variables|Default|GetType))
  (switch int _type
    (:Default
      (Sprite|SetFlipbook _sprite "/Game/SunnyLandAssets/sprites/player/run/tortoise-run.tortoise-run" :!label _label)
      (switch int _type
        (:Default
          (if (Variables|Default|GetState)
            _
            (else
              (bind _output_get (LocalVariables|SetRotation "0.000000,180.000000,0.000000" :!label _label_2)))))
        (:1
          (goto _label_2))
        (:2
          (goto _label_2)))
      (Transformation|SetRelativeRotation _sprite _output_get false false))
    (:2
      (if (Variables|Default|GetState)
        (Sprite|SetFlipbook _sprite "/Game/SunnyLandAssets/sprites/player/idle/tortoise-idle.tortoise-idle")
        (else
          (goto _label))))))

(fn GetNewSpeed
  (bind _basespeed (Variables|Default|GetBaseSpeed))
  (if (Variables|Default|GetState)
    (switch int (Variables|Default|GetType)
      (:2
        (LocalVariables|SetNewSpeed (* _basespeed 0.0)))
      (:3
        (LocalVariables|SetNewSpeed (* _basespeed -1.0))))
    (else
      (LocalVariables|SetNewSpeed _basespeed)))
  (return (LocalVariables|GetNewSpeed)))

(fn UpdateState
  (if (!= (Variables|Default|GetType) 1)
    (Variables|Default|SetState (not (Variables|Default|GetState)))))

(fn GetLocationDelta
  (params (Speed :type Float%20%28double-precision%29) (Time :type Float%20%28double-precision%29))
  (return (* Speed Time (Math|Vector|MakeVector 1.0 0.0 0.0))))

(fn GetDistanceLeft
  (return (- (.X (Math|Vector|BreakVector (Transformation|GetActorLocation (Variables|Default|GetEndGoal)))) (.X (Math|Vector|BreakVector (Transformation|GetActorLocation))))))

(fn ResetTime
  (if (Variables|Default|GetState)
    (Variables|Default|SetTime 0.5)
    (else
      (Variables|Default|SetTime 1.0))))

(fn UpdateSoundTime
  (params (DeltaSeconds :type Float%20%28double-precision%29))
  (bind _returnvalue (Transformation|GetActorLocation))
  (bind _output_get (Variables|Default|SetSoundTime (- (Variables|Default|GetSoundTime) DeltaSeconds)))
  (if (< _output_get 0.0)
    (switch int (Variables|Default|GetType)
      (:Default
        (Variables|Default|SetSoundTime 0.5)
        (Audio|PlaySoundatLocation "/Game/Sounds/grass_que.grass_que" _returnvalue "0, 0, 0" 1.0 1.0 0.0 0 0 0 0))
      (:3
        (Variables|Default|SetSoundTime 0.3)
        (Audio|PlaySoundatLocation "/Game/Sounds/dungeon_que.dungeon_que" _returnvalue "0, 0, 0" 1.0 1.0 0.0 0 0 0 0)))))